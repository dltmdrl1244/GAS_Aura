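; Enemy melee attack ability that faces the combat target and plays a random tagged attack montage.
; The montage's gameplay event triggers a radius query at the matching combat socket, damaging non-friendly live players.
; Any hit fires one MeleeImpact gameplay cue carrying the montage tag, then the ability ends, as it does when the montage completes or aborts.
; A leftover-style debug sphere draws at half the query radius.
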(event `self.K2_ActivateAbility`
  (bind _returnvalue (`self.GetAvatarActorFromActorInfo`))
  (bind _returnvalue_2 (`self.GetAvatarActorFromActorInfo`))
  (set `self.HasHitTarget` false)
  (bind _returnvalue_3 (message `EnemyCombatInterface.GetCombatTarget` _returnvalue_2))
  (bind _ascombat_interface (cast `CombatInterface` _returnvalue_2))
  (`CombatInterface.UpdateFacingTargetLocation` _ascombat_interface (`Actor.K2_GetActorLocation` _returnvalue_3))
  (bind _returnvalue_4 (message `CombatInterface.GetAttackMontages` (`self.GetAvatarActorFromActorInfo`)))
  (bind _output_get (set `self.Tagged Montage` (`self.GetRandomTaggedMontage` _returnvalue_4)))
  (bind (_montage _montagetag _sockettag) (break `TaggedMontage` _output_get))
  (`AbilityTask_PlayMontageAndWait.CreatePlayMontageAndWaitProxy` "None" _montage 1.0 "None" false
    (:`then`
      (`AbilityTask_WaitGameplayEvent.WaitGameplayEvent` _montagetag null
        (:`EventReceived`
          (bind _returnvalue_5 (message `CombatInterface.GetCombatSocketLocation` _returnvalue _sockettag))
          (bind _output_get_2 (set `self.SocketLocation` _returnvalue_5))
          (`KismetSystemLibrary.DrawDebugSphere` _output_get_2 50.0 12 (struct :`R` 1.0 :`B` 0.369039 :`A` 1.0) 1.0)
          (bind _outoverlappingactors (`AuraAbilitySystemLibrary.GetLivePlayersWithinRadius` _returnvalue (`|MakeArray` _returnvalue) 100.0 (`self.SocketLocation`)))
          (for _array_element _outoverlappingactors
            (bind _returnvalue_6 (`AuraAbilitySystemLibrary.IsFriendly` (`self.GetAvatarActorFromActorInfo`) _array_element))
            (if (not _returnvalue_6)
              (`self.CauseDamage` _array_element)
              (set `self.HasHitTarget` true)
              (message `CombatInterface.GetHitEffect` _array_element)))
          (if (`self.HasHitTarget`)
            (bind _returnvalue_7 (message `EnemyCombatInterface.GetCombatTarget` (`self.GetAvatarActorFromActorInfo`)))
            (`self.K2_ExecuteGameplayCueWithParams` (struct :`TagName` "GameplayCue.MeleeImpact") (`AbilitySystemBlueprintLibrary.MakeGameplayCueParameters` 0.0 0.0 (struct) (struct) (struct) (`BlueprintGameplayTagLibrary.MakeGameplayTagContainerFromTag` (`.MontageTag` (break `TaggedMontage` (`self.Tagged Montage`)))) (struct) (`self.SocketLocation`) (0.0 0.0 0.0) null (`self.GetAvatarActorFromActorInfo`) _returnvalue_7)))
          (`self.K2_EndAbility`))))
    (:`OnCompleted`
      (`self.K2_EndAbility` :!label _label))
    (:`OnInterrupted`
      (goto _label))
    (:`OnCancelled`
      (goto _label))))