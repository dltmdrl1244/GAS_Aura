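; BP_FireBolt is the actor for the Fire Bolt ability, with cleanup for bolts left dangling.
; Each tick it compares its current location with the one saved on the previous frame.
; When the distance moved falls below MinDistance, it spawns a Niagara fire explosion at that spot and destroys itself.
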(event `self.ReceiveTick`
  (params (DeltaSeconds :type "Float (single-precision)"))
  (`self.HandleDanglingFireBolt`))

(fn `HandleDanglingFireBolt`
  (set `self.LocationLastFrame` (`self.LocationThisFrame`))
  (set `self.LocationThisFrame` (`self.K2_GetActorLocation`))
  (if (< (`KismetMathLibrary.VSize` (- (`self.LocationLastFrame`) (`self.LocationThisFrame`))) (`self.MinDistance`))
    (`NiagaraFunctionLibrary.SpawnSystemAtLocation` "/Game/Assets/Effects/Projectiles/FireExplosion/NS_FireExplosion2.NS_FireExplosion2" (`self.LocationThisFrame`))
    (`self.K2_DestroyActor`)))

(fn `UserConstructionScript`)