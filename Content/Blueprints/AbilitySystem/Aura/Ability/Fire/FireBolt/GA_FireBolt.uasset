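; GA_FireBolt is a gameplay ability that casts homing fire bolt projectiles at the location under the cursor.
; On activation it commits, reads cursor target data, turns the avatar toward the hit location and plays the cast montage.
; A montage gameplay event triggers spawning from the weapon socket with an overridden launch pitch, homing on the hit actor.
; The ability ends when the montage completes, blends out or is interrupted or cancelled.
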(event `self.K2_ActivateAbility`
  (`self.K2_CommitAbility`)
  (bind (_asynctaskproxy _datahandle) (`TargetDataUnderCursor.CreateTargetDataUnderCursor`)
    (:`ValidData`
      (bind (_bblockinghit _binitialoverlap _time _distance _location _impactpoint _normal _impactnormal _physmat _hitactor) (`GameplayStatics.BreakHitResult` (`AbilitySystemBlueprintLibrary.GetHitResultFromTargetData` _datahandle)))
      (set `self.Projectile Target Location` _location)
      (set `self.MouseHitActor` _hitactor)
      (message `CombatInterface.UpdateFacingTargetLocation` (`self.GetAvatarActorFromActorInfo`) (`self.Projectile Target Location`))
      (`AbilityTask_PlayMontageAndWait.CreatePlayMontageAndWaitProxy` "None" "/Game/Assets/Characters/Aura/Animations/Abilities/AM_Cast_FireBolt.AM_Cast_FireBolt" 1.0 "None" false
        (:`then`
          (`AbilityTask_WaitGameplayEvent.WaitGameplayEvent` (struct :`TagName` "Event.Montage.FireBolt") null true
            (:`EventReceived`
              (`self.SpawnProjectiles` (`self.Projectile Target Location`) (`BlueprintGameplayTagLibrary.MakeLiteralGameplayTag` (struct :`TagName` "CombatSocket.Weapon")) true 25.0 (`self.MouseHitActor`)))))
        (:`OnCompleted`
          (`self.K2_EndAbility` :!label _label))
        (:`OnBlendOut`
          (goto _label))
        (:`OnInterrupted`
          (goto _label))
        (:`OnCancelled`
          (goto _label))))))

(event `self.K2_OnEndAbility`
  (params (bWasCancelled :type Boolean)))